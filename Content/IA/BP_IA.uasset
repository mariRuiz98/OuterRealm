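; BP_IA is an AI pawn Blueprint that wanders randomly and chases the player when it sees one.
; On BeginPlay it moves to random reachable navmesh points around itself, picking a new one each time a move succeeds.
; PawnSensing sightings start a move toward player zero and retrigger a one-second delay, after which it resumes wandering once sightings stop.
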(event OnSeePawn(PawnSensing)
  (params (Pawn :type Pawn%20Object%20Reference))
  ;[1 1 1] IA Detect Player
  (Utilities|FlowControl|Sequence
    (:then_0
      (Development|PrintString "Siguiendo al jugador")
      (AI|AIMoveTo self "0, 0, 0" (Game|Player|GetPlayerPawn 0) 5.0 false))
    (:then_1
      (Utilities|FlowControl|RetriggerableDelay 1.0)
      (CallFunction|GotoRandomPoint))))

(event Custom|GoToRandom%20Point
  ;[1 1 1] Movimiento IA Puntos Aleatorios
  (AI|AIMoveTo self (.RandomLocation (AI|Navigation|GetRandomReachablePointinRadius (Transformation|GetActorLocation) 1e+03 0 0)) 0 5.0 false
    (:OnSuccess
      (CallFunction|GotoRandomPoint))))

(event EventBeginPlay
  (CallFunction|GotoRandomPoint))

(fn ConstructionScript)